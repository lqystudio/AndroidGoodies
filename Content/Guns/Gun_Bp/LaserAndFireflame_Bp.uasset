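; LaserAndFireflame_Bp is a gun Blueprint, named for laser and flamethrower weapons, that handles the effects of a continuous-fire weapon.
; WeaponActivate shows and activates MuzzleParticles and starts FireSound, while WeaponDeactivate stops both and hides the particles.
; Both events print debug strings, and the graph contains no damage, trace or projectile logic.
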(event EventWeaponDeactivate
  (bind _muzzle_particles (Variables|Default|GetMuzzle_Particles))
  (Development|PrintString "deactve")
  (Components|Activation|Deactivate (Variables|Default|GetFireSound))
  (Components|Activation|Deactivate _muzzle_particles)
  (Rendering|SetVisibility _muzzle_particles false false))

(event EventWeaponActivate
  (Rendering|SetVisibility (Variables|Default|GetMuzzle_Particles) true false)
  (Development|PrintString "active")
  (Components|Activation|Activate (Variables|Default|GetFireSound) false)
  (Components|Activation|Activate (Variables|Default|GetMuzzle_Particles) false))

(fn ConstructionScript)